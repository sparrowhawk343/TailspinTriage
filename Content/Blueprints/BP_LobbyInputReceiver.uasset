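; Per-player lobby input receiver that handles joining, helicopter selection and readying up.
; Start registers the player with stat tracking, spawns and possesses a BP_FlyingCube display actor, and has GM_Lobby show the selection widget.
; Left/Right inputs cycle the widget's choice and refresh the actor's material.
; Ready rejects choices already taken and requires four connected players, then broadcasts the choice and removes the widget.
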(event Custom|MenuLeft
  (bind _characterselectwidgetref (Variables|Default|GetCharacterSelectWidgetRef))
  ;[1 1 1] Input for navigating left and right in select menu
  (Utilities|IsValid _characterselectwidgetref
    (:Is%20Valid
      (Default|SwitchCharacter _characterselectwidgetref -1)
      (CallFunction|SwitchCharacterColor))))

(event Custom|MenuRight
  (bind _characterselectwidgetref (Variables|Default|GetCharacterSelectWidgetRef))
  ;[1 1 1] Input for navigating left and right in select menu
  (Utilities|IsValid _characterselectwidgetref
    (:Is%20Valid
      (Default|SwitchCharacter _characterselectwidgetref 1)
      (CallFunction|SwitchCharacterColor))))

(event Custom|Ready
  (if (Variables|Default|GetbPlayerConnected)
    (bind _returnvalue (CallFunction|CompareCharacterChoice))
    (if _returnvalue
      (Development|PrintString "You cannot select the same helicopter as another player")
      (elif (>= (Variables|/Script/FG21FT_GP4_Team05.GP4_StatTrackingSubsystem|GetConnectedPlayersAmount (Subsystems|GetGP4StatTrackingSubsystem)) 4)
        (Utilities|FlowControl|DoOnce false
          (:Completed
            (Variables|Default|SetbReadyToPlay true)
            (Default|CallOnIsReadyChanged (Variables|/Game/Widgets/WBP_CharacterSelect.WBP_CharacterSelect_C|GetCharacterChoice (Variables|Default|GetCharacterSelectWidgetRef)))
            ;[1 1 1] Remove the widget and the ref to it.
            (Widget|RemovefromParent (Variables|Default|GetCharacterSelectWidgetRef))
            (Variables|Default|SetCharacterSelectWidgetRef 0)))
        (else
          (Development|PrintString "You have to be 4 players to play" true true "(R=0.000000,G=0.244062,B=0.369792,A=1.000000)" 1e+01))))
    (else
      (Development|PrintString "Connect with enter/start!"))))

(event Custom|Start
  (bind _playerindex (Variables|Default|GetPlayerIndex))
  (bind _playerindex_2 (Variables|Default|GetPlayerIndex))
  (Utilities|FlowControl|DoOnce false
    (:Completed
      (Variables|Default|SetbPlayerConnected true)
      ;[1 1 1] Adds player and info to the struct array in the game instance.
      (Default|CallOnPlayerConnected)
      (bind _asbp_gp_4game_instance (Utilities|Casting|CastToBP_Gp4GameInstance (Game|GetGameInstance))
        (:then
          (Variables|Default|SetGameInstance _asbp_gp_4game_instance)
          (Utilities|IsValid _asbp_gp_4game_instance
            (:Is%20Valid
              (Class|GP4StatTrackingSubsystem|SetUpPlayersData (Subsystems|GetGP4StatTrackingSubsystem) (Variables|Default|GetPlayerIndex))
              ;[1 1 1] Spawn the display character and set default choice.
              (bind _asgm_lobby (Utilities|Casting|CastToGM_Lobby (Game|GetGameMode)))
              (bind _returnvalue (Game|SpawnActorfromClass "/Game/Blueprints/BP_FlyingCube.BP_FlyingCube_C" (Transformation|GetActorTransform (Utilities|Array|Get(acopy) (Variables|/Game/Blueprints/GM_Lobby.GM_Lobby_C|GetPlayerStartArray _asgm_lobby) _playerindex_2)) "AdjustIfPossibleButAlwaysSpawn" 0 _playerindex_2 self))
              (Default|SetInstigator _returnvalue)
              (Pawn|Possess (Game|GetPlayerController _playerindex_2) _returnvalue)
              (Variables|Default|SetPlayerChoiceActor _returnvalue)
              (Class|GP4StatTrackingSubsystem|SetPlayerChoice (Subsystems|GetGP4StatTrackingSubsystem) _playerindex _playerindex)
              ;[1 1 1] Securesthe character selection widget is displayed, has to happen after players default character choice is set.
              (Utilities|IsValid (Variables|Default|GetCharacterSelectWidgetRef)
                (:Is%20Not%20Valid
                  (bind _asgm_lobby_2 (Utilities|Casting|CastToGM_Lobby (Game|GetGameMode)))
                  (Default|DisplayCharacterSelect _asgm_lobby_2 (Variables|Default|GetPlayerIndex))
                  ;[1 1 1] Visually display choice
                  (Default|SetPlayerMaterial (Variables|Default|GetPlayerChoiceActor)))))
            (:Is%20Not%20Valid
              (Development|PrintString "Invalid GameInstance!"))))
        (:CastFailed
          (Development|PrintString "Cast failed!"))))))

(event Input|ActionEvents|InputActionStart
  (params (Key :type Key%20Structure :default "None"))
  (bind _playerindex (Variables|Default|GetPlayerIndex))
  (bind _playerindex_2 (Variables|Default|GetPlayerIndex))
  (:Pressed
    (Utilities|FlowControl|DoOnce false
      (:Completed
        (Variables|Default|SetbPlayerConnected true)
        ;[1 1 1] Adds player and info to the struct array in the game instance.
        (Default|CallOnPlayerConnected)
        (bind _asbp_gp_4game_instance (Utilities|Casting|CastToBP_Gp4GameInstance (Game|GetGameInstance))
          (:then
            (Variables|Default|SetGameInstance _asbp_gp_4game_instance)
            (Utilities|IsValid _asbp_gp_4game_instance
              (:Is%20Valid
                (Class|GP4StatTrackingSubsystem|SetUpPlayersData (Subsystems|GetGP4StatTrackingSubsystem) (Variables|Default|GetPlayerIndex))
                ;[1 1 1] Spawn the display character and set default choice.
                (bind _asgm_lobby (Utilities|Casting|CastToGM_Lobby (Game|GetGameMode)))
                (bind _returnvalue (Game|SpawnActorfromClass "/Game/Blueprints/BP_FlyingCube.BP_FlyingCube_C" (Transformation|GetActorTransform (Utilities|Array|Get(acopy) (Variables|/Game/Blueprints/GM_Lobby.GM_Lobby_C|GetPlayerStartArray _asgm_lobby) _playerindex_2)) "AdjustIfPossibleButAlwaysSpawn" 0 _playerindex_2 self))
                (Default|SetInstigator _returnvalue)
                (Pawn|Possess (Game|GetPlayerController _playerindex_2) _returnvalue)
                (Variables|Default|SetPlayerChoiceActor _returnvalue)
                (Class|GP4StatTrackingSubsystem|SetPlayerChoice (Subsystems|GetGP4StatTrackingSubsystem) _playerindex _playerindex)
                ;[1 1 1] Securesthe character selection widget is displayed, has to happen after players default character choice is set.
                (Utilities|IsValid (Variables|Default|GetCharacterSelectWidgetRef)
                  (:Is%20Not%20Valid
                    (bind _asgm_lobby_2 (Utilities|Casting|CastToGM_Lobby (Game|GetGameMode)))
                    (Default|DisplayCharacterSelect _asgm_lobby_2 (Variables|Default|GetPlayerIndex))
                    ;[1 1 1] Visually display choice
                    (Default|SetPlayerMaterial (Variables|Default|GetPlayerChoiceActor)))))
              (:Is%20Not%20Valid
                (Development|PrintString "Invalid GameInstance!"))))
          (:CastFailed
            (Development|PrintString "Cast failed!")))))))

(event Input|ActionEvents|InputActionReady
  (params (Key :type Key%20Structure :default "None"))
  (:Pressed
    (if (Variables|Default|GetbPlayerConnected)
      (bind _returnvalue (CallFunction|CompareCharacterChoice))
      (if _returnvalue
        (Development|PrintString "You cannot select the same helicopter as another player")
        (elif (>= (Variables|/Script/FG21FT_GP4_Team05.GP4_StatTrackingSubsystem|GetConnectedPlayersAmount (Subsystems|GetGP4StatTrackingSubsystem)) 4)
          (Utilities|FlowControl|DoOnce false
            (:Completed
              (Variables|Default|SetbReadyToPlay true)
              (Default|CallOnIsReadyChanged (Variables|/Game/Widgets/WBP_CharacterSelect.WBP_CharacterSelect_C|GetCharacterChoice (Variables|Default|GetCharacterSelectWidgetRef)))
              ;[1 1 1] Remove the widget and the ref to it.
              (Widget|RemovefromParent (Variables|Default|GetCharacterSelectWidgetRef))
              (Variables|Default|SetCharacterSelectWidgetRef 0)))
          (else
            (Development|PrintString "You have to be 4 players to play" true true "(R=0.000000,G=0.244062,B=0.369792,A=1.000000)" 1e+01))))
      (else
        (Development|PrintString "Connect with enter/start!")))))

(event Input|ActionEvents|InputActionMenuLeft
  (params (Key :type Key%20Structure :default "None"))
  (bind _characterselectwidgetref (Variables|Default|GetCharacterSelectWidgetRef))
  ;[1 1 1] Input for navigating left and right in select menu
  (:Pressed
    (Utilities|IsValid _characterselectwidgetref
      (:Is%20Valid
        (Default|SwitchCharacter _characterselectwidgetref -1)
        (CallFunction|SwitchCharacterColor)))))

(event Input|ActionEvents|InputActionMenuRight
  (params (Key :type Key%20Structure :default "None"))
  (bind _characterselectwidgetref (Variables|Default|GetCharacterSelectWidgetRef))
  ;[1 1 1] Input for navigating left and right in select menu
  (:Pressed
    (Utilities|IsValid _characterselectwidgetref
      (:Is%20Valid
        (Default|SwitchCharacter _characterselectwidgetref 1)
        (CallFunction|SwitchCharacterColor)))))

(fn ConstructionScript)

(fn SwitchCharacterColor
  ;[1 1 1] Visual set material according to player choice.
  (Default|SetPlayerMaterial (Variables|Default|GetPlayerChoiceActor)))

(fn CompareCharacterChoice
  (bind _characterselectwidgetref (Variables|Default|GetCharacterSelectWidgetRef))
  (bind _characterchoice (Variables|/Game/Widgets/WBP_CharacterSelect.WBP_CharacterSelect_C|GetCharacterChoice _characterselectwidgetref))
  (bind _asgm_lobby (Utilities|Casting|CastToGM_Lobby (Game|GetGameMode)))
  (if (< (Utilities|Array|FindItem (Variables|/Game/Blueprints/GM_Lobby.GM_Lobby_C|GetReadyCharacterChoices _asgm_lobby) _characterchoice) 0)
    (LocalVariables|SetYesNo false)
    (elif (== _characterchoice (Utilities|Array|Get(acopy) (Variables|/Game/Blueprints/GM_Lobby.GM_Lobby_C|GetReadyCharacterChoices _asgm_lobby) (Utilities|Array|FindItem (Variables|/Game/Blueprints/GM_Lobby.GM_Lobby_C|GetReadyCharacterChoices _asgm_lobby) _characterchoice)))
      (LocalVariables|SetYesNo true)
      (else
        (LocalVariables|SetYesNo false))))
  (return (LocalVariables|GetYesNo)))