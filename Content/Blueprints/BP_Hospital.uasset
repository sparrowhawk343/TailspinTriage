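; BP_Hospital is a player's goal building, colored with the team material of that player's chosen character.
; On BeginPlay it uses HospitalIndex to fetch player data from the GP4 stat tracking subsystem.
; The character choice keys into the game instance's lookup, supplying the material for the Hospital and Logo meshes.
; The logo starts at a random yaw and spins steadily on Tick.
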(event EventBeginPlay
  (bind _hospital (Variables|Default|GetHospital))
  ;[1 1 1] Set goal color after player character choice.
  (bind _asbp_gp_4game_instance (Utilities|Casting|CastToBP_Gp4GameInstance (Game|GetGameInstance)))
  (bind _output_get (Variables|Default|SetGameInstance _asbp_gp_4game_instance))
  (bind _returnvalue (Class|GP4StatTrackingSubsystem|GetPlayerData (Subsystems|GetGP4StatTrackingSubsystem) (Variables|Default|GetHospitalIndex)))
  (Rendering|Material|SetMaterial _hospital 0 (Variables|/Script/FG21FT_GP4_Team05.GP4_CharacterData|GetTeamMaterial (.Value (Utilities|Map|Find (Variables|/Script/FG21FT_GP4_Team05.GP4_CharacterLookUp|GetCharacterLookUp (Variables|/Game/Blueprints/BP_Gp4GameInstance.BP_Gp4GameInstance_C|GetCharacterLookUp _output_get)) (.CharacterChoice (Utilities|Struct|BreakPlayerData _returnvalue))))))
  (Rendering|Material|SetMaterial _hospital 1 (Variables|/Script/FG21FT_GP4_Team05.GP4_CharacterData|GetTeamMaterial (.Value (Utilities|Map|Find (Variables|/Script/FG21FT_GP4_Team05.GP4_CharacterLookUp|GetCharacterLookUp (Variables|/Game/Blueprints/BP_Gp4GameInstance.BP_Gp4GameInstance_C|GetCharacterLookUp _output_get)) (.CharacterChoice (Utilities|Struct|BreakPlayerData _returnvalue))))))
  (Rendering|Material|SetMaterial (Variables|Default|GetLogo) 0 (Variables|/Script/FG21FT_GP4_Team05.GP4_CharacterData|GetTeamMaterial (.Value (Utilities|Map|Find (Variables|/Script/FG21FT_GP4_Team05.GP4_CharacterLookUp|GetCharacterLookUp (Variables|/Game/Blueprints/BP_Gp4GameInstance.BP_Gp4GameInstance_C|GetCharacterLookUp _output_get)) (.CharacterChoice (Utilities|Struct|BreakPlayerData _returnvalue))))))
  (Transformation|AddLocalRotation (Variables|Default|GetLogo) (Math|Rotator|MakeRotator 0.0 0.0 (Math|Random|RandomFloatinRange 0.0 359.0)) false false))

(event Collision|EventActorBeginOverlap
  (params (OtherActor :type Actor%20Object%20Reference)))

(event EventTick
  (params (DeltaSeconds :type Float%20%28single-precision%29))
  (Transformation|AddLocalRotation (Variables|Default|GetLogo) (Math|Rotator|MakeRotator 0.0 0.0 (* DeltaSeconds 2e+01)) false false))

(fn ConstructionScript)