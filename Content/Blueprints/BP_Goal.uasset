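; Player-owned helipad goal that scores patient chain cubes delivered during a versus round.
; On BeginPlay it colors zone and helipad by the owner's character, sets up its score widget and registers with the game instance.
; Overlaps before time runs out play money effects and credit attached flyers with undamaged rescues or other-goal deliveries via the stat subsystem.
; The goal owner receives the patient's value, then the cube is destroyed and game mode and UI update.
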(event EventBeginPlay
  ;[1 1 1] Set goal color after player character choice.
  (bind _asbp_gp_4game_instance (Utilities|Casting|CastToBP_Gp4GameInstance (Game|GetGameInstance)))
  (bind _output_get (Variables|Default|SetGameInstance _asbp_gp_4game_instance))
  (bind _returnvalue (Class|GP4StatTrackingSubsystem|GetPlayerData (Subsystems|GetGP4StatTrackingSubsystem) (Variables|Default|GetGoalIndex)))
  (Rendering|Material|SetMaterial (Variables|Default|GetZone) 0 (Variables|/Script/FG21FT_GP4_Team05.GP4_CharacterData|GetGoalMaterial (.Value (Utilities|Map|Find (Variables|/Script/FG21FT_GP4_Team05.GP4_CharacterLookUp|GetCharacterLookUp (Variables|/Game/Blueprints/BP_Gp4GameInstance.BP_Gp4GameInstance_C|GetCharacterLookUp _output_get)) (.CharacterChoice (Utilities|Struct|BreakPlayerData _returnvalue))))))
  (Rendering|Material|SetMaterial (Variables|Default|GetHelipad) 0 (Variables|/Script/FG21FT_GP4_Team05.GP4_CharacterData|GetTeamMaterial (.Value (Utilities|Map|Find (Variables|/Script/FG21FT_GP4_Team05.GP4_CharacterLookUp|GetCharacterLookUp (Variables|/Game/Blueprints/BP_Gp4GameInstance.BP_Gp4GameInstance_C|GetCharacterLookUp _output_get)) (.CharacterChoice (Utilities|Struct|BreakPlayerData _returnvalue))))))
  (bind _asui_goal_score (Utilities|Casting|CastToUI_GoalScore (UserInterface|GetUserWidgetObject (Variables|Default|GetWidget))))
  (Variables|/Game/Widgets/UI_GoalScore.UI_GoalScore_C|SetPlayerIndex _asui_goal_score (Variables|Default|GetGoalIndex))
  (Utilities|Array|AddUnique (Variables|/Game/Blueprints/BP_Gp4GameInstance.BP_Gp4GameInstance_C|GetGoals (Variables|Default|GetGameInstance)) self))

(event Collision|EventActorBeginOverlap
  (params (OtherActor :type Actor%20Object%20Reference))
  (bind _returnvalue (Subsystems|GetGP4StatTrackingSubsystem))
  (bind _goalindex (Variables|Default|GetGoalIndex))
  (if (not (Variables|/Script/FG21FT_GP4_Team05.GP4_TimerSubsystem|GetbTimerRunOut (Subsystems|GetGP4TimerSubsystem)))
    (if (Utilities|DoesObjectImplementInterface OtherActor "/Game/Blueprints/BPI_ChainCube.BPI_ChainCube_C")
      (Audio|PlaySound2D "/Game/Audio/SFX/goal_money_kashing.goal_money_kashing" 1.0 1.0 0.0 0 0)
      (Niagara|SpawnSystematLocation "/Game/Particles/NS_Money.NS_Money" (+ (Transformation|GetWorldLocation (Variables|Default|GetHelipad)) "0,0,400.000000"))
      ;[1 1 1] Loop through the players attached and update either score on other goal or roundscore.
      (Utilities|IsValid OtherActor
        (:Is%20Valid
          (bind _asbp_chain_cube (Utilities|Casting|CastToBP_ChainCube OtherActor))
          (for _array_element (Variables|/Game/Blueprints/BP_ChainCube.BP_ChainCube_C|GetAttachedActorArray _asbp_chain_cube)
            (bind _asbp_flying_cube (Utilities|Casting|CastToBP_FlyingCube _array_element))
            (if (Variables|/Game/Blueprints/BP_ChainCube.BP_ChainCube_C|GetDamaged _asbp_chain_cube)
              _
              (else
                (Class|GP4StatTrackingSubsystem|UpdateHealthyPatientsRescued _returnvalue (Variables|/Game/Blueprints/BP_FlyingCube.BP_FlyingCube_C|GetIndex _asbp_flying_cube))))
            (if (!= (Variables|/Game/Blueprints/BP_FlyingCube.BP_FlyingCube_C|GetIndex _asbp_flying_cube) _goalindex)
              (Class|GP4StatTrackingSubsystem|UpdateScoreinOtherPlayersGoal _returnvalue (Variables|/Game/Blueprints/BP_FlyingCube.BP_FlyingCube_C|GetIndex _asbp_flying_cube) _goalindex)))
          (Class|GP4StatTrackingSubsystem|UpdatePlayerRoundScore _returnvalue _goalindex (Variables|/Game/Blueprints/BP_ChainCube.BP_ChainCube_C|GetPatientValue _asbp_chain_cube))
          (Class|BPIChainCube|Destroy(Message) OtherActor true)
          (bind _asgm_versus (Utilities|Casting|CastToGM_Versus (Game|GetGameMode)))
          (Default|PlayerScored _asgm_versus)
          ;[1 1 1] Update this goals score and update UI
          (Default|CallOnUpdateScoreUI (Variables|Default|GetGoalIndex)))))))

(fn ConstructionScript)