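; Versus game mode that runs local multiplayer rounds, from player spawning to score and winner screens.
; On BeginPlay it spawns a possessed flying cube per connected player, sharing one camera, and creates the UI.
; Chain cubes launch randomly from cycling spawn points initially and whenever a player scores or patient dies.
; Timer expiry banks round scores through the stat subsystem and shows results; the GameInstance's game-end event opens the winner screen.
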(event Custom|PlayerScored
  (CallFunction|SpawnBalls 1))

(event Custom|OnTimerRanOut
  (bind _returnvalue (Subsystems|GetGP4StatTrackingSubsystem))
  (bind _roundsscorescreen (Variables|Default|GetRoundsScoreScreen))
  ;[1 1 1] When time is out add the round score and reset for next round. Has to happen before the round score creen is added.
  (Class|GP4StatTrackingSubsystem|AddAllPlayersRoundScoretoRound _returnvalue)
  (Class|GP4StatTrackingSubsystem|ResetAllPlayersCurrentRoundScore _returnvalue)
  (Class|GP4StatTrackingSubsystem|UpdatePlayersTotalScore _returnvalue)
  (Widget|SetVisibility (Variables|Default|GetHUDRef) "Collapsed")
  (UserInterface|Viewport|AddtoViewport _roundsscorescreen 0)
  (Default|OpenScreen _roundsscorescreen))

(event Custom|OnGameEnd
  (bind _winnerscreen (Variables|Default|GetWinnerScreen))
  ;[1 1 1] Create the winner screen and bind event to on game end so it shows the winner screen then. Put in own func when working.
  (UserInterface|Viewport|AddtoViewport _winnerscreen 0)
  (Default|OpenScreen _winnerscreen))

(event Custom|PatientKilled
  (CallFunction|SpawnBalls 1))

(event Custom|InitialPatientsSpawn
  (Utilities|FlowControl|Delay 2.0)
  (CallFunction|SpawnBalls 2))

(event EventBeginPlay
  (bind _outactors (Actor|GetAllActorsOfClass "/Game/Blueprints/BP_Camera.BP_Camera_C"))
  (Variables|Default|SetCameraRef (Utilities|Array|Get(acopy) _outactors))
  (CallFunction|GetPlayerStartPoints)
  (CallFunction|SpawnPlayersfromLobby)
  (CallFunction|GetBallSpawnPoints)
  (CallFunction|InitialPatientsSpawn)
  (CallFunction|CreatePlayerScores)
  (Input|EnableInput (Game|GetPlayerController 0))
  (CallFunction|GameStarted)
  (Development|ExecuteConsoleCommand "t.maxfps 60" 0)
  ;[1 1 1] Add the HUD with display scores widget
  (bind _returnvalue (UserInterface|CreateWidget "/Game/Widgets/WBP_HUD.WBP_HUD_C"))
  (bind _output_get (Variables|Default|SetHUDRef _returnvalue))
  (UserInterface|Viewport|AddtoViewport _output_get 0)
  (bind _returnvalue_2 (UserInterface|CreateWidget "/Game/Widgets/WBP_RoundScoresScreen.WBP_RoundScoresScreen_C"))
  (Variables|Default|SetRoundsScoreScreen _returnvalue_2)
  (EventDispatchers|BindEventtoOnTimerRanOut (Subsystems|GetGP4TimerSubsystem) (delegate Custom|OnTimerRanOut))
  ;[1 1 1] Create the winner screen and bind event to on game end so it shows the winner screen then. Put in own func when working.
  (bind _returnvalue_3 (UserInterface|CreateWidget "/Game/Widgets/WBP_WinScreen.WBP_WinScreen_C"))
  (Variables|Default|SetWinnerScreen _returnvalue_3)
  (bind _asbp_gp_4game_instance (Utilities|Casting|CastToBP_Gp4GameInstance (Game|GetGameInstance)))
  (EventDispatchers|BindEventtoOnGameEnd _asbp_gp_4game_instance (delegate Custom|OnGameEnd)))

(event Input|KeyboardEvents|F
  (params (Key :type Key%20Structure :default "None")))

(event Input|KeyboardEvents|Escape
  (params (Key :type Key%20Structure :default "None"))
  (:Pressed
    (Game|QuitGame 0 "Quit" false)))

(fn ConstructionScript)

(fn GetPlayerStartPoints
  (bind _outactors (Actor|GetAllActorsOfClass "/Script/Engine.PlayerStart"))
  (Variables|Default|SetPlayerStartArray _outactors))

(fn SpawnInputReceivers
  (for (_ _array_index) (Variables|Default|GetPlayerStartArray)
    (LocalVariables|SetIndex _array_index)
    (for _array_element (Variables|Default|GetPlayerStartArray)
      (if (== (CallFunction|NametoInt _array_element) (LocalVariables|GetIndex))
        (Class|GameplayStatics|CreatePlayer -1)
        (bind _returnvalue (Game|SpawnActorfromClass "/Game/Blueprints/BP_InputReceiver.BP_InputReceiver_C" (Transformation|GetActorTransform (Utilities|Array|Get(acopy) (Variables|Default|GetPlayerStartArray) (LocalVariables|GetIndex))) "Undefined" 0 (LocalVariables|GetIndex) 0))
        (Utilities|Array|AddUnique (Variables|Default|GetPlayerInputReceiverArray) _returnvalue)
        (Pawn|Possess (Game|GetPlayerController (LocalVariables|GetIndex)) _returnvalue)
        (Utilities|Array|AddUnique (Variables|Default|GetPlayerControllerArray) (Game|GetPlayerController (LocalVariables|GetIndex)))))))

(fn NametoInt
  (params (PlayerStart :type Player%20Start%20Object%20Reference))
  (return (Math|Conversions|ToInteger(Byte) (Utilities|String|ToString(Name) (Variables|/Script/Engine.PlayerStart|GetPlayerStartTag PlayerStart)))))

(fn GetBallSpawnPoints
  (bind _outactors (Actor|GetAllActorsOfClass "/Game/Blueprints/BP_BallSpawnPoint.BP_BallSpawnPoint_C"))
  (Variables|Default|SetBallSpawnPointArray _outactors))

(fn SpawnBalls
  (params (SpawnAmount :type Integer))
  (for _index (range 1 SpawnAmount)
    (bind _returnvalue (Game|SpawnActorfromClass "/Game/Blueprints/BP_ChainCube.BP_ChainCube_C" (Transformation|GetActorTransform (Utilities|Array|Get(acopy) (Variables|Default|GetBallSpawnPointArray) (Variables|Default|GetCurrentBallSpawnIndex))) "AdjustIfPossibleButAlwaysSpawn" 0 0 0))
    (Transformation|SetWorldRotation (Variables|/Game/Blueprints/BP_ChainCube.BP_ChainCube_C|GetChainCube _returnvalue) (Math|Random|RandomRotator true) false false)
    (Physics|AddImpulse (Variables|/Game/Blueprints/BP_ChainCube.BP_ChainCube_C|GetChainCube _returnvalue) (* (Math|Random|RandomUnitVector) 1e+04) "None" false)
    (bind _result (Math|Integer|IncrementInt (Variables|Default|GetCurrentBallSpawnIndex))
      (:%20%20
        (if (> _result 3)
          (Variables|Default|SetCurrentBallSpawnIndex 0))))))

(fn CreatePlayerScores
  (for _index (range 0 3)
    (Utilities|Array|Add (Variables|Default|GetPlayerScores) (Utilities|Struct|MakePlayerScores _index))))

(fn AddPlayerScore
  (params (ScoreToAdd :type Integer) (PlayerIndex :type Integer))
  (bind _playerscores (Variables|Default|GetPlayerScores))
  (Utilities|Struct|SetmembersinPlayerScores (Utilities|Array|Get(acopy) _playerscores PlayerIndex) (+ ScoreToAdd (.playerscore (Utilities|Array|Get(acopy) _playerscores PlayerIndex)))))

(fn GetPlayerScore
  (params (PlayerIndex :type Integer))
  (return (.playerscore (Utilities|Array|Get(acopy) (Variables|Default|GetPlayerScores) PlayerIndex))))

(fn SpawnPlayersfromLobby
  (Utilities|Array|Clear (Variables|Default|GetPlayers))
  (bind _asbp_gp_4game_instance (Utilities|Casting|CastToBP_Gp4GameInstance (Game|GetGameInstance)))
  (for _index (range 0 (- (Variables|/Game/Blueprints/BP_Gp4GameInstance.BP_Gp4GameInstance_C|GetConnectedPlayers _asbp_gp_4game_instance) 1))
    (bind _returnvalue (Game|SpawnActorfromClass "/Game/Blueprints/BP_FlyingCube.BP_FlyingCube_C" (Transformation|GetActorTransform (Utilities|Array|Get(acopy) (Variables|Default|GetPlayerStartArray) _index)) "Undefined" 0 _index 0))
    (Utilities|Array|Add (Variables|Default|GetPlayers) _returnvalue)
    (Pawn|Possess (Game|GetPlayerController _index) _returnvalue)
    (Game|Player|SetViewTargetwithBlend (Game|GetPlayerController _index) (Variables|Default|GetCameraRef) 0.0 "VTBlend_Linear" 0.0 false))
  (CallFunction|RemoveUnusedCameras)
  (return))

(fn GameStarted
  (Variables|Default|SetbIsInGame true)
  (Default|GameStarted (Variables|Default|GetCameraRef) (Variables|Default|GetPlayers)))

(fn RemoveUnusedCameras
  (bind _outactors (Actor|GetAllActorsOfClass "/Script/Engine.CameraActor"))
  (for _array_element _outactors
    (Actor|DestroyActor _array_element)))

(fn SpawnPlayer
  (params (CurrentPlayerIndex :type Integer) (InputReceiver :type BP%20Input%20Receiver%20Object%20Reference))
  (bind _returnvalue (Game|SpawnActorfromClass "/Game/Blueprints/BP_FlyingCube.BP_FlyingCube_C" (Transformation|GetActorTransform InputReceiver) "Undefined" 0 CurrentPlayerIndex 0))
  (Pawn|Possess (Game|GetPlayerController CurrentPlayerIndex) _returnvalue)
  (return false))