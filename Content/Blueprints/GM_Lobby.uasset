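; Lobby game mode that sets up local multiplayer character selection and starts the game once connected players are ready.
; On BeginPlay it creates local players at tag-indexed PlayerStarts, each possessing a BP_LobbyInputReceiver registered with the game instance.
; Receiver events update the connected-player count and trigger ready checks that call ProceedGame on the game instance.
; Helper functions, not called here, link character-select widgets to receivers and spawn possessed BP_FlyingCube pawns.
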(event Custom|IncreaseConnectedPlayers
  ;[1 1 1] Event listeners
  (CallFunction|AddConnectedPlayer))

(event Custom|CheckIfReady
  (params (CharacterChoice :type Integer))
  ;[1 1 1] Event listeners
  (CallFunction|CheckifReadytoPlay CharacterChoice))

(event EventBeginPlay
  (Input|EnableInput (Game|GetPlayerController 0))
  (CallFunction|GetPlayerStartPoints)
  (CallFunction|SpawnInputReceivers)
  (Development|ExecuteConsoleCommand "t.maxfps 60" 0)
  ;[1 1 1] Event listeners
  (for _array_element (Variables|Default|GetPlayerInputReceiverArray)
    (EventDispatchers|BindEventtoOnIsReadyChanged _array_element (delegate Custom|CheckIfReady))
    (EventDispatchers|BindEventtoOnPlayerConnected _array_element (delegate Custom|IncreaseConnectedPlayers))
    ;[1 1 1] Adds the widget that hold the character selection widgets.
    (bind _returnvalue (UserInterface|CreateWidget "/Game/Widgets/WBP_SelectMenu.WBP_SelectMenu_C"))
    (bind _output_get (Variables|Default|SetSelectWidgetReference _returnvalue))
    (UserInterface|Viewport|AddtoViewport _output_get 0)))

(event Input|KeyboardEvents|Escape
  (params (Key :type Key%20Structure :default "None"))
  (:Pressed
    (Game|QuitGame 0 "Quit" false)))

(fn ConstructionScript)

(fn GetPlayerStartPoints
  (bind _outactors (Actor|GetAllActorsOfClass "/Script/Engine.PlayerStart"))
  (Variables|Default|SetPlayerStartArray _outactors))

(fn SpawnInputReceivers
  (for (_ _array_index) (Variables|Default|GetPlayerStartArray)
    (LocalVariables|SetIndex _array_index)
    (for _array_element (Variables|Default|GetPlayerStartArray)
      (if (== (CallFunction|NametoInt _array_element) (LocalVariables|GetIndex))
        (Class|GameplayStatics|CreatePlayer -1)
        (bind _returnvalue (Game|SpawnActorfromClass "/Game/Blueprints/BP_LobbyInputReceiver.BP_LobbyInputReceiver_C" (Transformation|GetActorTransform (Utilities|Array|Get(acopy) (Variables|Default|GetPlayerStartArray) (LocalVariables|GetIndex))) "Undefined" 0 (LocalVariables|GetIndex) false 0 0))
        (Utilities|Array|AddUnique (Variables|Default|GetPlayerInputReceiverArray) _returnvalue)
        ;[1 1 1] Add number of input recivers to the game instance array
        (bind _asbp_gp_4game_instance (Utilities|Casting|CastToBP_Gp4GameInstance (Game|GetGameInstance)))
        (Utilities|Array|AddUnique (Variables|/Game/Blueprints/BP_Gp4GameInstance.BP_Gp4GameInstance_C|GetPlayerInputRecivers _asbp_gp_4game_instance) _returnvalue)
        (Pawn|Possess (Game|GetPlayerController (LocalVariables|GetIndex)) _returnvalue)
        (Utilities|Array|AddUnique (Variables|Default|GetPlayerControllerArray) (Game|GetPlayerController (LocalVariables|GetIndex)))))))

(fn NametoInt
  (params (PlayerStart :type Player%20Start%20Object%20Reference))
  (return (Math|Conversions|ToInteger(Byte) (Utilities|String|ToString(Name) (Variables|/Script/Engine.PlayerStart|GetPlayerStartTag PlayerStart)))))

(fn CheckifReadytoPlay
  (params (CharacterChoice :type Integer))
  (Utilities|Array|AddUnique (Variables|Default|GetReadyCharacterChoices) CharacterChoice)
  (for _index (range 0 (- (Variables|Default|GetConnectedPlayers) 1))
    (if (not (Variables|/Game/Blueprints/BP_LobbyInputReceiver.BP_LobbyInputReceiver_C|GetbReadyToPlay (Utilities|Array|Get(acopy) (Variables|Default|GetPlayerInputReceiverArray) _index)))
      (return)))
  (bind _asbp_gp_4game_instance (Utilities|Casting|CastToBP_Gp4GameInstance (Game|GetGameInstance))
    (:then
      (Default|ProceedGame _asbp_gp_4game_instance))
    (:CastFailed
      (Development|PrintString "cast to bp g4 game instance failed!"))))

(fn DisplayCharacterSelect
  (params (CurrentPlayerIndex :type Integer))
  (bind _characterselect (Default|AddCharacterSelect (Variables|Default|GetSelectWidgetReference) CurrentPlayerIndex))
  ;[1 1 1 1 12] Bind to inputs from the input reciver when selecting.
  (Variables|/Game/Blueprints/BP_LobbyInputReceiver.BP_LobbyInputReceiver_C|SetCharacterSelectWidgetRef (Utilities|Array|Get(acopy) (Variables|Default|GetPlayerInputReceiverArray) CurrentPlayerIndex) _characterselect)
  (return))

(fn AddConnectedPlayer
  ;[1 1 1] Set the number of players variable both in this BP and the game instance.
  (bind _output_get (Variables|Default|SetConnectedPlayers (+ (Variables|Default|GetConnectedPlayers) 1)))
  (bind _asbp_gp_4game_instance (Utilities|Casting|CastToBP_Gp4GameInstance (Game|GetGameInstance)))
  (Variables|/Game/Blueprints/BP_Gp4GameInstance.BP_Gp4GameInstance_C|SetConnectedPlayers _asbp_gp_4game_instance _output_get))

(fn SpawnPlayer
  (params (CurrentPlayerIndex :type Integer) (InputReceiver :type BP%20Input%20Receiver%20Object%20Reference))
  (bind _returnvalue (Game|SpawnActorfromClass "/Game/Blueprints/BP_FlyingCube.BP_FlyingCube_C" (Transformation|GetActorTransform InputReceiver) "Undefined" 0 CurrentPlayerIndex 0))
  (Pawn|Possess (Game|GetPlayerController CurrentPlayerIndex) _returnvalue)
  (return false))