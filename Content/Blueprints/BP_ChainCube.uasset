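; Physics-driven patient on a gurney for versus mode that flying cubes attach to and that registers with GM_Versus for camera tracking.
; Hits above a speed threshold, except against bumpable or chain-cube actors, cost health after a spawn grace period and between cooldowns.
; Half health doubles patient value and loops a material flash.
; Detaching flags a steal to remaining cubes; death notifies attached actors and the game mode, then destroys it.
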(event Custom|DamageCooldownTimer
  (if (Variables|Default|GetCanTakeDamage)
    (Variables|Default|SetCanTakeDamage false)
    (Utilities|FlowControl|Delay (Variables|Default|GetDamageCooldown))
    (Variables|Default|SetCanTakeDamage true)))

(event Custom|DamageBufferDelay
  ;[1 1 1] Damage buffer when patient spawns
  (Utilities|FlowControl|Delay 3.0)
  (Variables|Default|SetCanTakeDamage true))

(event Custom|DamageFX
  (bind _chaincube (Variables|Default|GetChainCube))
  (Audio|PlaySound2D "/Game/Audio/SFX/SFX_Patient_Hurt.SFX_Patient_Hurt" 1.0 1.0 0.0 0 0 false)
  (bind _returnvalue (Niagara|SpawnSystematLocation "/Game/AssetPacks/StylizedFireEffects/FX/NS_FlashHit.NS_FlashHit" (Transformation|GetWorldLocation _chaincube) (Transformation|GetWorldRotation _chaincube) "0.500000,0.500000,0.500000"))
  (Class|NiagaraComponent|SetCustomTimeDilation _returnvalue 1.0)
  (CallFunction|DamageFlash))

(event Custom|DeathFX
  (bind _chaincube (Variables|Default|GetChainCube))
  (bind _returnvalue (Niagara|SpawnSystematLocation "/Game/AssetPacks/StylizedFireEffects/FX/NS_HitEffect.NS_HitEffect" (Transformation|GetWorldLocation _chaincube) (Transformation|GetWorldRotation _chaincube)))
  (Class|NiagaraComponent|SetCustomTimeDilation _returnvalue 2.5))

(event Custom|StartDamageFlashLoop
  (bind _value (Timeline|Timeline_DamageFlashLoop Play)
    (:Update
      (Rendering|Material|SetScalarParameterValue (Variables|Default|GetGurneyDynamicMaterial) "FlashValue" _value :!class /Script/Engine.MaterialInstanceDynamic))))

(event Custom|DamageFlash
  (bind _value (Timeline|Timeline_DamageFlash Play)
    (:Update
      (Rendering|Material|SetScalarParameterValue (Variables|Default|GetGurneyDynamicMaterial) "FlashValue" _value :!class /Script/Engine.MaterialInstanceDynamic))))

(event Custom|SpawnFX
  (bind _chaincube (Variables|Default|GetChainCube))
  (bind _returnvalue (Niagara|SpawnSystematLocation "/Game/AssetPacks/StylizedFireEffects/FX/NS_HitEffect.NS_HitEffect" (Transformation|GetWorldLocation _chaincube) (Transformation|GetWorldRotation _chaincube)))
  (Class|NiagaraComponent|SetCustomTimeDilation _returnvalue 2.0)
  (Audio|PlaySound2D "/Game/Audio/SFX/pop.pop" 0.3 1.0 0.0 0 0))

(event EventDetach
  (params (AttachedActor :type Actor%20Object%20Reference))
  (bind _attachedactorarray (Variables|Default|GetAttachedActorArray))
  (Utilities|Array|RemoveItem _attachedactorarray AttachedActor)
  (for _array_element _attachedactorarray
    (bind _asbp_flying_cube (Utilities|Casting|CastToBP_FlyingCube _array_element))
    (Utilities|IsValid _asbp_flying_cube
      (:Is%20Valid
        (Default|UpdatePatientStolen _asbp_flying_cube)))))

(event EventAttach
  (params (AttachedActor :type Actor%20Object%20Reference))
  (Utilities|Array|AddUnique (Variables|Default|GetAttachedActorArray) AttachedActor))

(event EventDestroy
  (params (IsGoal :type Boolean))
  (for _array_element (Variables|Default|GetAttachedActorArray)
    (Class|BPIChainBreak|ChainBreak(Message) _array_element IsGoal))
  (CallFunction|RemovefromCameraTracking)
  (Actor|DestroyActor))

(event EventTick
  (params (DeltaSeconds :type Float%20%28single-precision%29))
  (CallFunction|GetCurrentVelocity))

(event Collision|EventHit
  (params (MyComp :type Primitive%20Component%20Object%20Reference) (Other :type Actor%20Object%20Reference) (OtherComp :type Primitive%20Component%20Object%20Reference) (bSelfMoved :type Boolean) (HitLocation :type Vector :default "0, 0, 0") (HitNormal :type Vector :default "0, 0, 0") (NormalImpulse :type Vector :default "0, 0, 0") (Hit :type Hit%20Result%20Structure%20%28by%20ref%29))
  (CallFunction|DamageCheck Other))

(event EventBeginPlay
  (Variables|Default|SetCurrentHealth (Variables|Default|GetMaxHealth))
  (CallFunction|DamageBufferDelay)
  (bind _aswbp_patient_health_bar (Utilities|Casting|CastToWBP_PatientHealthBar (UserInterface|GetUserWidgetObject (Variables|Default|GetHealthBar))))
  (bind _output_get (Variables|Default|SetHealthBarWidget _aswbp_patient_health_bar))
  (Variables|/Game/Widgets/WBP_PatientHealthBar.WBP_PatientHealthBar_C|SetHealth _output_get (Variables|Default|GetCurrentHealth))
  (CallFunction|AddtoCameraTracking)
  (bind _returnvalue (Rendering|Material|CreateDynamicMaterialInstance (Variables|Default|GetGurney) 0 "/Game/AssetPacks/Gurney/Gurney_Color3.Gurney_Color3" "None" :!class /Script/Engine.PrimitiveComponent))
  (Variables|Default|SetGurneyDynamicMaterial _returnvalue)
  (bind _returnvalue_2 (Actor|GetActorOfClass "/Game/Blueprints/BP_Camera.BP_Camera_C"))
  (Utilities|IsValid _returnvalue_2
    (:Is%20Valid
      (Variables|Default|SetCamera _returnvalue_2)
      (CallFunction|SpawnFX))))

(fn ConstructionScript)

(fn GetCurrentVelocity
  (bind _returnvalue (Physics|GetPhysicsLinearVelocity (Variables|Default|GetChainCube) "None"))
  (Variables|Default|SetCurrentVelocity (Math|Vector|VectorLength _returnvalue)))

(fn DamageCheck
  (params (OtherActor :type Actor%20Object%20Reference))
  (bind _attachedactorarray (Variables|Default|GetAttachedActorArray))
  (if (Variables|Default|GetCanTakeDamage)
    (if (and (> (Variables|Default|GetCurrentVelocity) (Variables|Default|GetDamageVelocityThreshold)) (Math|Boolean|NORBoolean (Utilities|DoesObjectImplementInterface OtherActor "/Game/Blueprints/BPI_Bumpable.BPI_Bumpable_C") (Utilities|DoesObjectImplementInterface OtherActor "/Game/Blueprints/BPI_ChainCube.BPI_ChainCube_C")))
      (bind _result (Math|Integer|DecrementInt (Variables|Default|GetCurrentHealth))
        (:%20%20
          (CallFunction|DamageFX)
          (Variables|/Game/Widgets/WBP_PatientHealthBar.WBP_PatientHealthBar_C|SetHealth (Variables|Default|GetHealthBarWidget) _result)
          (if (== (Variables|Default|GetCurrentHealth) (/ (Variables|Default|GetMaxHealth) 2))
            (Variables|Default|SetPatientValue (* (Variables|Default|GetPatientValue) 2)) ; If health is 50%, double patient value
            (Variables|Default|SetDamaged true)
            (CallFunction|StartDamageFlashLoop))
          (if (<= (Variables|Default|GetCurrentHealth) 0)
            (if (Utilities|Array|IsNotEmpty _attachedactorarray)
              (for _array_element _attachedactorarray
                (Class|BPIChainBreak|PatientKilled(Message) _array_element)))
            (bind _asgm_versus (Utilities|Casting|CastToGM_Versus (Game|GetGameMode)))
            (Default|PatientKilled _asgm_versus)
            (CallFunction|DeathFX)
            (CallFunction|Destroy false)
            (else
              (CallFunction|DamageCooldownTimer))))))))

(fn AddtoCameraTracking
  (bind _asgm_versus (Utilities|Casting|CastToGM_Versus (Game|GetGameMode)))
  (Utilities|Array|Add (Variables|/Game/Blueprints/GM_Versus.GM_Versus_C|GetPatients _asgm_versus) self))

(fn RemovefromCameraTracking
  (bind _asgm_versus (Utilities|Casting|CastToGM_Versus (Game|GetGameMode)))
  (Utilities|Array|RemoveItem (Variables|/Game/Blueprints/GM_Versus.GM_Versus_C|GetPatients _asgm_versus) self))