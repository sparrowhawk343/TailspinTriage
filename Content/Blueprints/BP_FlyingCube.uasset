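; Player helicopter pawn that flies on physics thrusters, picks up patients on a breakable chain and bumps other players.
; Axis input drives lift, weakened by ground distance, and turn thrust; Tick adds fall compensation, lean, rotor blur and a traced shadow.
; Pickup overlap attaches a physics constraint and cable through BPI_ChainCube; bumps knock the pawn and break its chain.
; It also forwards menu input to the lobby receiver and reports match stats.
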(event OnConstraintBroken(Chain)
  (params (ConstraintIndex :type Integer))
  (CallFunction|BreakChain false))

(event OnComponentBeginOverlap(Patient_Pickup_Radius)
  (params (OverlappedComponent :type Primitive%20Component%20Object%20Reference) (OtherActor :type Actor%20Object%20Reference) (OtherComp :type Primitive%20Component%20Object%20Reference) (OtherBodyIndex :type Integer) (bFromSweep :type Boolean) (SweepResult :type Hit%20Result%20Structure%20%28by%20ref%29))
  (CallFunction|CubeAttachCheck OtherActor) ; Check for cube, attach
)

(event Custom|TimerRanOutHandler
  ;[1 1 1] Setup
  (CallFunction|TimerRanOut))

(event Custom|AttachCooldownTimer
  (if (Variables|Default|GetCanAttach)
    (Variables|Default|SetCanAttach false)
    (Utilities|FlowControl|Delay (Variables|Default|GetBallAttachCooldown))
    (Variables|Default|SetCanAttach true)))

(event Custom|UpdateRotateThruster_Turn
  (bind _thruster_rotate_turn (Variables|Default|GetThruster_Rotate_Turn))
  (bind _maxrotatethrust (Variables|Default|GetMaxRotateThrust))
  (bind _thruster_rotate_turn1 (Variables|Default|GetThruster_Rotate_Turn1))
  ;[1 1 1] Activate auto thrusters, if you're not using your main thrusters
  (if (== (Variables|Default|GetThrustStrength_Turn) 0.0)
    (Variables|/Script/Engine.PhysicsThrusterComponent|SetThrustStrength _thruster_rotate_turn _maxrotatethrust)
    (Variables|/Script/Engine.PhysicsThrusterComponent|SetThrustStrength _thruster_rotate_turn1 _maxrotatethrust)
    (else
      (Variables|/Script/Engine.PhysicsThrusterComponent|SetThrustStrength _thruster_rotate_turn 0.0)
      (Variables|/Script/Engine.PhysicsThrusterComponent|SetThrustStrength _thruster_rotate_turn1 0.0))))

(event Custom|TimerRanOut
  (Class|GP4StatTrackingSubsystem|UpdateTimeHoldingPatient (Subsystems|GetGP4StatTrackingSubsystem) (Variables|Default|GetIndex) (Variables|Default|GetTimeHeldPatient)))

(event Custom|BumpCooldownTimer
  (if (Variables|Default|GetCanBeBumped)
    (Variables|Default|SetCanBeBumped false)
    (Utilities|FlowControl|Delay (Variables|Default|GetBumpCooldown))
    (Variables|Default|SetCanBeBumped true)))

(event Custom|UpdateTimeHeldPatient
  (if (Variables|Default|GetAttached)
    (Utilities|FlowControl|Delay 1.0)
    (Math|Integer|IncrementInt (Variables|Default|GetTimeHeldPatient))))

(event Custom|UpdatePatientStolen
  (Class|GP4StatTrackingSubsystem|UpdatePatientsStolen (Subsystems|GetGP4StatTrackingSubsystem) (Variables|Default|GetIndex)))

(event EventBeginPlay
  ;[1 1 1] Setup
  (bind _asgp4_game_instance (Utilities|Casting|CastToGP4_GameInstance (Game|GetGameInstance)))
  (Variables|Default|SetAttachedBall 0)
  (CallFunction|SetPlayerMaterial)
  (Class|GP4GameInstance|AddPlayer _asgp4_game_instance self)
  (EventDispatchers|BindEventtoOnTimerRanOut (Subsystems|GetGP4TimerSubsystem) (delegate Custom|TimerRanOutHandler))
  (bind _returnvalue (Rendering|Material|CreateDynamicMaterialInstance (Variables|Default|GetRotor) 0 "/Game/AssetPacks/Helicopter/RotorMat.RotorMat" "None" :!class /Script/Engine.PrimitiveComponent))
  (Variables|Default|SetRotorDynamicMaterial _returnvalue))

(event EventChainBreak
  (params (IsGoal :type Boolean))
  (CallFunction|BreakChain IsGoal)
  (Class|PhysicsConstraintComponent|BreakConstraint (Variables|Default|GetChain)))

(event EventBump
  (params (Direction :type Vector :default "0, 0, 0") (Velocity :type Float%20%28double-precision%29))
  (bind _cube (Variables|Default|GetCube))
  (if (Variables|Default|GetCanBeBumped)
    (CallFunction|BumpCooldownTimer)
    (Physics|AddImpulse _cube (* Direction (* Velocity (Variables|Default|GetBumpForceMultiplier))) "None" false)
    (bind _returnvalue (Niagara|SpawnSystematLocation "/Game/AssetPacks/StylizedFireEffects/FX/NS_Impact02.NS_Impact02" (Transformation|GetWorldLocation _cube) (Transformation|GetWorldRotation _cube) "3.000000,3.000000,3.000000"))
    (Class|NiagaraComponent|SetCustomTimeDilation _returnvalue 1.25)
    (CallFunction|ChainBreak false)))

(event Collision|EventHit
  (params (MyComp :type Primitive%20Component%20Object%20Reference) (Other :type Actor%20Object%20Reference) (OtherComp :type Primitive%20Component%20Object%20Reference) (bSelfMoved :type Boolean) (HitLocation :type Vector :default "0, 0, 0") (HitNormal :type Vector :default "0, 0, 0") (NormalImpulse :type Vector :default "0, 0, 0") (Hit :type Hit%20Result%20Structure%20%28by%20ref%29))
  ;[1 1 1] Collision checks
  (CallFunction|PlayerBumpCheck OtherComp Other) ; Check for player, bump
  (CallFunction|EnvironmentBounce (.normal Hit)) ; If neither, bounce on environment
)

(event EventTick
  (params (DeltaSeconds :type Float%20%28single-precision%29))
  (CallFunction|GroundCheck)
  (CallFunction|GetCurrentVelocity)
  (CallFunction|ThrusterFX)
  (CallFunction|UpdateRotateThrusterTurn)
  (CallFunction|VerticalThrusterCompensation)
  (CallFunction|UpdateShadowLocation)
  (CallFunction|UpdateTimeHeldPatient)
  (CallFunction|UpdateForwardLean)
  (CallFunction|RotateRotor))

(event EventPatientKilled
  (Class|GP4StatTrackingSubsystem|UpdatePatientsKilled (Subsystems|GetGP4StatTrackingSubsystem) (Variables|Default|GetIndex)))

(event Input|ActionEvents|InputActionMenuLeft
  (params (Key :type Key%20Structure :default "None"))
  (bind _lobbyinputreceiver (Variables|Default|GetLobbyInputReceiver))
  ;[1 1 1] Send lobby inputs to LobbyInputReceiver
  (:Pressed
    (Utilities|IsValid _lobbyinputreceiver
      (:Is%20Valid
        (Default|MenuLeft _lobbyinputreceiver)))))

(event Input|ActionEvents|InputActionMenuRight
  (params (Key :type Key%20Structure :default "None"))
  (bind _lobbyinputreceiver (Variables|Default|GetLobbyInputReceiver))
  ;[1 1 1] Send lobby inputs to LobbyInputReceiver
  (:Pressed
    (Utilities|IsValid _lobbyinputreceiver
      (:Is%20Valid
        (Default|MenuRight _lobbyinputreceiver)))))

(event Input|ActionEvents|InputActionStart
  (params (Key :type Key%20Structure :default "None"))
  (bind _lobbyinputreceiver (Variables|Default|GetLobbyInputReceiver))
  ;[1 1 1] Send lobby inputs to LobbyInputReceiver
  (:Pressed
    (Utilities|IsValid _lobbyinputreceiver
      (:Is%20Valid
        (Default|Start _lobbyinputreceiver)))))

(event Input|ActionEvents|InputActionReady
  (params (Key :type Key%20Structure :default "None"))
  (bind _lobbyinputreceiver (Variables|Default|GetLobbyInputReceiver))
  ;[1 1 1] Send lobby inputs to LobbyInputReceiver
  (:Pressed
    (Utilities|IsValid _lobbyinputreceiver
      (:Is%20Valid
        (Default|Ready _lobbyinputreceiver)))))

(event Input|ActionEvents|InputActionThrust
  (params (Key :type Key%20Structure :default "None"))
  ;[1 1 1] Bounce the player up when they thrust close to the ground
)

(event Input|AxisEvents|InputAxisThrust_Turn
  (params (AxisValue :type Float%20%28single-precision%29))
  (bind _thruster_turn (Variables|Default|GetThruster_Turn))
  ;[1 1 1] Setting Thrust strength with input
  (Utilities|DeadZone AxisValue 0.05
    (:True
      (Variables|/Script/Engine.PhysicsThrusterComponent|SetThrustStrength _thruster_turn (Math|Float|Lerp 0.0 (Variables|Default|GetMaxTurnThrust) AxisValue))
      ;[1 1 1] Change propeller sound volume (Em spaget)
      (Variables|Default|SetThrustStrengthForwardZero false)
      (Audio|Components|Audio|SetVolumeMultiplier (Variables|Default|Gethelicopter_propeller_active) (/ (+ (stale Input|AxisEvents|InputAxisThrust AxisValue) 0.5) 1.0) :!class /Script/Engine.AudioComponent))
    (:False
      (Variables|/Script/Engine.PhysicsThrusterComponent|SetThrustStrength _thruster_turn 0.0)
      (bind _output_get (Variables|Default|SetThrustStrengthForwardZero true)))))

(event Input|AxisEvents|InputAxisThrust
  (params (AxisValue :type Float%20%28single-precision%29))
  (bind _grounddistance (Variables|Default|GetGroundDistance))
  (bind _thruster_bottom (Variables|Default|GetThruster_Bottom))
  (bind _maxthrust (Variables|Default|GetMaxThrust))
  (bind _helicopter_propeller_active (Variables|Default|Gethelicopter_propeller_active))
  (bind _returnvalue (Math|Float|Lerp 0.0 _maxthrust AxisValue))
  (bind _returnvalue_2 (* _grounddistance 38.0))
  (bind _returnvalue_3 (- _returnvalue _returnvalue_2))
  ;[1 1 1] Setting Thrust strength with input
  (Utilities|DeadZone AxisValue 0.05
    (:True
      (if (> _returnvalue_3 0.0)
        (Variables|/Script/Engine.PhysicsThrusterComponent|SetThrustStrength _thruster_bottom _returnvalue_3)
        ;[1 1 1] Change propeller sound volume (Em spaget)
        (Variables|Default|SetThrustStrengthUpZero false)
        (Audio|Components|Audio|SetVolumeMultiplier _helicopter_propeller_active (/ (+ AxisValue 0.5) 1.0) :!class /Script/Engine.AudioComponent)
        (else
          (Variables|/Script/Engine.PhysicsThrusterComponent|SetThrustStrength _thruster_bottom 0.0 :!label _label)
          (bind _output_get (Variables|Default|SetThrustStrengthUpZero true))
          (if (and _output_get (stale Input|AxisEvents|InputAxisThrust_Turn _output_get))
            (Audio|Components|Audio|SetVolumeMultiplier _helicopter_propeller_active 0.2 :!class /Script/Engine.AudioComponent)))))
    (:False
      (goto _label))))

(fn ConstructionScript)

(fn AttachChain
  (params (_Actor :type Actor%20Object%20Reference))
  (bind _thruster_bottom (Variables|Default|GetThruster_Bottom))
  (Variables|Default|SetAttached true)
  (Variables|Default|SetAttachedBall _Actor)
  (Class|PhysicsConstraintComponent|SetConstrainedComponents (Variables|Default|GetChain) (Variables|Default|GetCube) "None" (Actor|GetComponentbyClass _Actor "/Script/Engine.StaticMeshComponent") "None")
  (Class|CableComponent|SetAttachEndto (Variables|Default|GetCable) _Actor "ChainCube" "Center")
  (Effects|SpawnEmitterAttached "/Game/Particles/P_SparksBig.P_SparksBig" _thruster_bottom "None" (Transformation|GetWorldLocation _thruster_bottom) (Transformation|GetWorldRotation _thruster_bottom) "1.000000,1.000000,1.000000" "KeepWorldPosition")
  (Audio|PlaySound2D "/Game/Audio/SFX/SFX_Cable_Attach.SFX_Cable_Attach" 1.0 1.0 0.0 0 0))

(fn BreakChain
  (params (IsGoal :type Boolean))
  (bind _thruster_bottom (Variables|Default|GetThruster_Bottom))
  (if IsGoal
    (bind _returnvalue (Niagara|SpawnSystematLocation "/Game/AssetPacks/StylizedFireEffects/FX/NS_Impact04.NS_Impact04" (Transformation|GetWorldLocation _thruster_bottom) (Transformation|GetWorldRotation _thruster_bottom) "2.000000,2.000000,2.000000"))
    (Class|NiagaraComponent|SetCustomTimeDilation _returnvalue 1.25)
    (else
      (Utilities|IsValid (Variables|Default|GetAttachedBall)
        (:Is%20Valid
          (Class|BPIChainCube|Detach(Message) (Variables|Default|GetAttachedBall) self)
          (Class|GP4StatTrackingSubsystem|UpdateTimesCordBroke (Subsystems|GetGP4StatTrackingSubsystem) (Variables|Default|GetIndex))
          (Audio|PlaySound2D "/Game/Audio/SFX/SFX_Cable_Break.SFX_Cable_Break" 1.0 1.0 0.0 0 0 false)))))
  (Variables|Default|SetAttached false)
  (Variables|Default|SetAttachedBall 0)
  (Class|CableComponent|SetAttachEndto (Variables|Default|GetCable) self "Cube" "None")
  (CallFunction|AttachCooldownTimer))

(fn Bounce
  (bind _cube (Variables|Default|GetCube))
  (bind _jumpforce (Variables|Default|GetJumpForce))
  (if (Variables|Default|GetGrounded)
    (Utilities|FlowControl|Sequence
      (:then_0
        (Physics|AddImpulse _cube (Math|Vector|MakeVector 0.0 0.0 _jumpforce) "None" false))
      (:then_1
        (Physics|AddImpulseatLocation _cube (Math|Vector|MakeVector 0.0 0.0 (/ _jumpforce 2.0)) (Transformation|GetWorldLocation (Variables|Default|GetThruster_Bottom)) "None")))))

(fn GroundCheck
  (bind _cube (Variables|Default|GetCube))
  (bind _returnvalue (Transformation|GetWorldLocation _cube))
  (bind (_outhit _returnvalue_2) (Collision|LineTraceByChannel _returnvalue (- _returnvalue (Math|Vector|MakeVector 0.0 0.0 (Variables|Default|GetGroundCheckDistance))) "TraceTypeQuery1" false 0 "None"))
  (if (and (not (Utilities|DoesObjectImplementInterface (.hitactor _outhit) "/Game/Blueprints/BPI_ChainCube.BPI_ChainCube_C")) (not (Utilities|DoesObjectImplementInterface (.hitactor _outhit) "/Game/Blueprints/BPI_ChainBreak.BPI_ChainBreak_C")))
    (Variables|Default|SetGrounded _returnvalue_2)
    (bind _output_get (Variables|Default|SetGroundDistance (Math|Vector|Distance(Vector) (.location _outhit) _returnvalue)))))

(fn ThrusterFX
  (bind _ns_thrust_bottom (Variables|Default|GetNS_Thrust_Bottom))
  (Variables|Default|SetThrustStrength_Bottom (Variables|/Script/Engine.PhysicsThrusterComponent|GetThrustStrength (Variables|Default|GetThruster_Bottom)))
  (Variables|Default|SetThrustStrength_Turn (Variables|/Script/Engine.PhysicsThrusterComponent|GetThrustStrength (Variables|Default|GetThruster_Turn)))
  (Utilities|DeadZone (Math|Float|MapRangeClamped (Variables|Default|GetThrustStrength_Bottom) 0.0 (Variables|Default|GetMaxThrust) 0.0 2.0) 1.0
    (:True
      (Components|Activation|SetActive _ns_thrust_bottom true false))
    (:False
      (Components|Activation|SetActive _ns_thrust_bottom false false))))

(fn SetPlayerMaterial
  (bind _asbp_gp_4game_instance (Utilities|Casting|CastToBP_Gp4GameInstance (Game|GetGameInstance)))
  (bind _returnvalue (Class|GP4StatTrackingSubsystem|GetPlayerData (Subsystems|GetGP4StatTrackingSubsystem) (Variables|Default|GetIndex)))
  (Rendering|Material|SetMaterial (Variables|Default|GetPlayerModel) 0 (Variables|/Script/FG21FT_GP4_Team05.GP4_CharacterData|GetTeamMaterial (.Value (Utilities|Map|Find (Variables|/Script/FG21FT_GP4_Team05.GP4_CharacterLookUp|GetCharacterLookUp (Variables|/Game/Blueprints/BP_Gp4GameInstance.BP_Gp4GameInstance_C|GetCharacterLookUp _asbp_gp_4game_instance)) (.CharacterChoice (Utilities|Struct|BreakPlayerData _returnvalue)))))))

(fn GetCurrentVelocity
  (bind _returnvalue (Physics|GetPhysicsLinearVelocity (Variables|Default|GetCube) "None"))
  (Variables|Default|SetCurrentVelocity (Math|Vector|VectorLength _returnvalue)))

(fn PlayerBumpCheck
  (params (OtherActorComp :type Scene%20Component%20Object%20Reference) (OtherActor :type Actor%20Object%20Reference))
  (bind _currentvelocity (Variables|Default|GetCurrentVelocity))
  (if (Math|Boolean|ANDBoolean (> _currentvelocity (Variables|Default|GetBumpSpeed)) (Utilities|DoesObjectImplementInterface OtherActor "/Game/Blueprints/BPI_Bumpable.BPI_Bumpable_C") (> (+ (Variables|Default|GetThrustStrength_Bottom) (Variables|Default|GetThrustStrength_Turn)) 1e+01))
    (Class|BPIBumpable|Bump(Message) OtherActor (Math|Vector|Normalize (- (Transformation|GetWorldLocation OtherActorComp) (Transformation|GetWorldLocation (Variables|Default|GetCube)))) _currentvelocity)
    (Audio|PlaySound2D "/Game/Audio/SFX/SFX_Helicopter_Bump_Player.SFX_Helicopter_Bump_Player" 1.0 1.0 0.0 0 0)
    ;[1 1 1] Stat tracking
    (Class|GP4StatTrackingSubsystem|UpdateTimesBumpedOtherPlayers (Subsystems|GetGP4StatTrackingSubsystem) (Variables|Default|GetIndex))))

(fn EnvironmentBounce
  (params (HitNormal :type Vector))
  (if (> (Variables|Default|GetCurrentVelocity) 1.0)
    (Physics|AddImpulse (Variables|Default|GetCube) (* HitNormal (Variables|Default|GetBounceForce)) "None" false)))

(fn CubeAttachCheck
  (params (OtherActor :type Actor%20Object%20Reference))
  (if (Math|Boolean|ANDBoolean (Utilities|DoesObjectImplementInterface OtherActor "/Game/Blueprints/BPI_ChainCube.BPI_ChainCube_C") (not (Variables|Default|GetAttached)) (Variables|Default|GetCanAttach))
    (Class|BPIChainCube|Attach(Message) OtherActor self)
    (CallFunction|AttachChain OtherActor)))

(fn SetInstigator
  (bind _asbp_lobby_input_receiver (Utilities|Casting|CastToBP_LobbyInputReceiver (Game|GetInstigator)))
  (Utilities|IsValid _asbp_lobby_input_receiver
    (:Is%20Valid
      (Variables|Default|SetLobbyInputReceiver _asbp_lobby_input_receiver))))

(fn VerticalThrusterCompensation
  (bind _thruster_bottom_compensation (Variables|Default|GetThruster_Bottom_Compensation))
  (bind _returnvalue (Physics|GetPhysicsLinearVelocity (Variables|Default|GetCube) "None"))
  (if (< (.z _returnvalue) -25.0)
    (bind _output_get (Variables|/Script/Engine.PhysicsThrusterComponent|SetThrustStrength _thruster_bottom_compensation (* (Math|Float|Absolute(Float) (.z _returnvalue)) (Variables|Default|GetVerticalCompensationMultiplier))))
    (else
      (Variables|/Script/Engine.PhysicsThrusterComponent|SetThrustStrength _thruster_bottom_compensation 0.0))))

(fn UpdateShadowLocation
  (bind _cube (Variables|Default|GetCube))
  (bind _returnvalue (Transformation|GetWorldLocation _cube))
  (bind (_outhit _returnvalue_2) (Collision|LineTraceByChannel _returnvalue (- _returnvalue "0,0,1500.000000") "TraceTypeQuery1" false 0 "None"))
  (if _returnvalue_2
    (Transformation|SetWorldLocation (Variables|Default|GetShadowDecal) (.location _outhit) false true)))

(fn UpdateForwardLean
  (bind _playercollider (Variables|Default|GetPlayerCollider))
  (bind _relativerotation (Variables|/Script/Engine.SceneComponent|GetRelativeRotation _playercollider))
  (Transformation|SetRelativeRotation _playercollider (Math|Rotator|MakeRotator (.roll _relativerotation) (.pitch (Math|Interpolation|RInterpTo (Variables|/Script/Engine.SceneComponent|GetRelativeRotation _playercollider) (Math|Rotator|MakeRotator (.roll _relativerotation) (Math|Float|MapRangeClamped (Variables|Default|GetThrustStrength_Turn) 0.0 (Variables|Default|GetMaxTurnThrust) 0.0 45.0) (.yaw _relativerotation)) (Utilities|Time|GetWorldDeltaSeconds) 3.5)) (.yaw _relativerotation)) false false))

(fn RotateRotor
  (bind _minrotorspeed (LocalVariables|GetMinRotorSpeed))
  (bind _thruststrength_bottom (Variables|Default|GetThrustStrength_Bottom))
  (bind _maxthrust (Variables|Default|GetMaxThrust))
  (bind _maxrotorspeed (LocalVariables|GetMaxRotorSpeed))
  (bind _returnvalue (Math|Float|MapRangeClamped _thruststrength_bottom 0.0 _maxthrust _minrotorspeed _maxrotorspeed))
  (Transformation|AddLocalRotation (Variables|Default|GetRotor) (Math|Rotator|MakeRotator 0.0 0.0 (* (* _returnvalue (Utilities|Time|GetWorldDeltaSeconds)) -1.0)) false false)
  (Rendering|Material|SetScalarParameterValue (Variables|Default|GetRotorDynamicMaterial) "Blur" (Math|Float|NormalizetoRange _returnvalue _minrotorspeed _maxrotorspeed) :!class /Script/Engine.MaterialInstanceDynamic))