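; Physics-driven, player-flown helicopter that picks up cube actors on a breakable chain.
; Input axes set thruster strength, compensated for tilt and mass, and apply yaw torque plus clamped self-levelling tilt torques, with center of mass aligned to the thruster.
; Hitting a cube attaches the constraint and cable via BPI_ChainCube; ChainBreak or constraint failure releases them with sparks.
; Other hits bounce the body; fin overlap only prints debug text.
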(event OnConstraintBroken(Chain)
  (params (ConstraintIndex :type Integer))
  (CallFunction|BreakChain))

(event OnComponentBeginOverlap(Fin_Forward)
  (params (OverlappedComponent :type Primitive%20Component%20Object%20Reference) (OtherActor :type Actor%20Object%20Reference) (OtherComp :type Primitive%20Component%20Object%20Reference) (OtherBodyIndex :type Integer) (bFromSweep :type Boolean) (SweepResult :type Hit%20Result%20Structure%20%28by%20ref%29))
  ;[1 1 1] Collision with the player and goal(for testing purposes). It technically works but needs to be refined in terms of collisions with the other player.
  (Utilities|Casting|CastToBP_FlyingCube OtherActor)
  (Development|PrintString "WOAH! i bumped into a player!!!"))

(event EventBeginPlay
  ;[1 1 1] Setup
  (Utilities|Casting|CastToBP_Gp4GameInstance (Game|GetGameInstance))
  (Rendering|Material|SetMaterial (Variables|Default|GetHelicopterBodyMesh) 0 0)
  (Variables|Default|SetAttachedBall 0)
  (|CenterOfMassOffsetFix))

(event EventChainBreak
  (CallFunction|BreakChain))

(event Collision|EventHit
  (params (MyComp :type Primitive%20Component%20Object%20Reference) (Other :type Actor%20Object%20Reference) (OtherComp :type Primitive%20Component%20Object%20Reference) (bSelfMoved :type Boolean) (HitLocation :type Vector :default "0, 0, 0") (HitNormal :type Vector :default "0, 0, 0") (NormalImpulse :type Vector :default "0, 0, 0") (Hit :type Hit%20Result%20Structure%20%28by%20ref%29))
  (bind _helicopterbodymesh (Variables|Default|GetHelicopterBodyMesh))
  (if (Utilities|String|Contains (Utilities|GetObjectName Other) "cube")
    (if (not (Variables|Default|GetAttached))
      (Class|BPIChainCube|Attach(Message) Other self)
      (CallFunction|AttachChain Other))
    (else
      ;[1 1 1] Environment hit
      (bind _returnvalue (Physics|GetPhysicsLinearVelocity _helicopterbodymesh "None"))
      (if (> (Math|Vector|VectorLength _returnvalue) 0.5)
        (Physics|AddImpulse _helicopterbodymesh (* (.normal Hit) (Variables|Default|GetBounceForce)) "None" false)))))

(event EventTick
  (params (DeltaSeconds :type Float%20%28single-precision%29))
  (CallFunction|GroundCheck))

(event Input|AxisEvents|InputAxisMoveUp
  (params (AxisValue :type Float%20%28single-precision%29))
  ;[1 1 1] Move Up/Down
  (Variables|/Script/Engine.PhysicsThrusterComponent|SetThrustStrength (Variables|Default|GetPhysicsThruster) (* (/ (+ (* AxisValue 1e+03) 9.7e+02) (.z (Transformation|GetActorUpVector))) (Physics|GetMass (Variables|Default|GetHelicopterBodyMesh)))))

(event Input|AxisEvents|InputAxisRotateRight
  (params (AxisValue :type Float%20%28single-precision%29))
  ;[1 1 1] Rotation
  (Class|PrimitiveComponent|AddTorqueinDegrees (Variables|Default|GetHelicopterBodyMesh) (* AxisValue (Transformation|GetActorUpVector) 6e+02) "None" true))

(event Input|AxisEvents|InputAxisTiltForward
  (params (AxisValue :type Float%20%28single-precision%29))
  ;[1 1 1] Tilt Forward
  (Class|PrimitiveComponent|AddTorqueinDegrees (Variables|Default|GetHelicopterBodyMesh) (* (Transformation|GetActorRightVector) (Math|Float|Clamp(Float) (+ (* AxisValue 3e+01) (.pitch (Transformation|GetWorldRotation (Variables|Default|GetHelicopterBodyMesh)))) -2e+01 2e+01) 5.0) "None" true))

(event Input|AxisEvents|InputAxisTiltRight
  (params (AxisValue :type Float%20%28single-precision%29))
  ;[1 1 1] Tilt Sideways
  (Class|PrimitiveComponent|AddTorqueinDegrees (Variables|Default|GetHelicopterBodyMesh) (* (Transformation|GetActorForwardVector) (Math|Float|Clamp(Float) (+ (* AxisValue -3e+01) (.roll (Transformation|GetWorldRotation (Variables|Default|GetHelicopterBodyMesh)))) -2e+01 2e+01) 5.0) "None" true))

(fn ConstructionScript)

(fn AttachChain
  (params (_Actor :type Actor%20Object%20Reference))
  (bind _scene (Variables|Default|GetScene))
  (if (and (not (Variables|Default|GetAttached)) (Utilities|DoesObjectImplementInterface _Actor "/Game/Blueprints/BPI_ChainCube.BPI_ChainCube_C"))
    (Variables|Default|SetAttached true)
    (Variables|Default|SetAttachedBall _Actor)
    (Class|PhysicsConstraintComponent|SetConstrainedComponents (Variables|Default|GetChain) (Variables|Default|GetHelicopterBodyMesh) "None" (Actor|GetComponentbyClass _Actor "/Script/Engine.StaticMeshComponent") "None")
    (Class|CableComponent|SetAttachEndto (Variables|Default|GetCable) _Actor "ChainCube" "None")
    (Effects|SpawnEmitterAttached "/Game/Particles/P_SparksBig.P_SparksBig" 0 "None" (Transformation|GetWorldLocation _scene) (Transformation|GetWorldRotation _scene) "1.000000,1.000000,1.000000" "KeepWorldPosition")))

(fn BreakChain
  (bind _scene (Variables|Default|GetScene))
  (Class|CableComponent|SetAttachEndto (Variables|Default|GetCable) self "Cube" "None")
  (Variables|Default|SetAttached false)
  (Variables|Default|SetAttachedBall 0)
  (Effects|SpawnEmitterAttached "/Game/Particles/P_SparksSnap.P_SparksSnap" 0 "None" (Transformation|GetWorldLocation _scene) (Transformation|GetWorldRotation _scene) "1.000000,1.000000,1.000000" "KeepWorldPosition"))

(fn Bounce
  (bind _helicopterbodymesh (Variables|Default|GetHelicopterBodyMesh))
  (bind _jumpforce (Variables|Default|GetJumpForce))
  (if (Variables|Default|GetGrounded)
    (Utilities|FlowControl|Sequence
      (:then_0
        (Physics|AddImpulse _helicopterbodymesh (Math|Vector|MakeVector 0.0 0.0 _jumpforce) "None" false))
      (:then_1
        (Physics|AddImpulseatLocation _helicopterbodymesh (Math|Vector|MakeVector 0.0 0.0 (/ _jumpforce 2.0)) (Transformation|GetWorldLocation (Variables|Default|GetScene)) "None")))))

(fn GroundCheck
  (bind _helicopterbodymesh (Variables|Default|GetHelicopterBodyMesh))
  (bind _returnvalue (Transformation|GetWorldLocation _helicopterbodymesh))
  (bind _returnvalue_2 (Collision|LineTraceByChannel _returnvalue (- _returnvalue (Math|Vector|MakeVector 0.0 0.0 (Variables|Default|GetGroundCheckDistance))) "TraceTypeQuery1" false 0 "None"))
  (Variables|Default|SetGrounded _returnvalue_2))