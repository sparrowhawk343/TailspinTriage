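; Game instance that runs a round-based game, choosing levels, persisting settings and playing background music.
; ProceedGame either fires the game-end event or starts a new round, which clears goals, opens the level mapped to the round number and starts the timer subsystem.
; Init sets the round and loads or creates the settings save object.
; LoadSettings loads the slot but discards the result, and EndOfRound is empty.
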(event EventInit
  (CallFunction|SetCurrentRound)
  (CallFunction|CreateSaveGameObject)
  (CallFunction|LoadSettings))

(fn LoadLevel
  (params (LevelToLoad :type Name))
  (Game|OpenLevel(byName) LevelToLoad))

(fn GetLeveltoLoad
  (bind _levelmap (Variables|Default|GetLevelMap))
  (bind _currentround (Variables|Default|GetCurrentRound))
  (bind (_value _returnvalue) (Utilities|Map|Find _levelmap _currentround))
  (if _returnvalue
    (return _value)
    (else
      (Development|PrintString "No level matching current round number."))))

(fn StartNewRound
  (Utilities|Array|Clear (Variables|Default|GetGoals))
  (bind _levelname (CallFunction|GetLeveltoLoad))
  (CallFunction|LoadLevel _levelname)
  (Class|GP4TimerSubsystem|StartTimer (Subsystems|GetGP4TimerSubsystem))
  (Default|CallOnStartNewRound))

(fn SetCurrentRound
  ;[1 1 1] If this is the first round set the current round to be the first. Could also always be set in init to 1?
  (if (<= (Variables|Default|GetCurrentRound) 0)
    (Variables|Default|SetCurrentRound 1)
    (else
      ;[1 1 1] If choose to play again and lobby loads it still uses same game instance? So we have to reset number of rounds to 1? This check is before the check what round it is.
      (if (> (Variables|Default|GetCurrentRound) (Variables|Default|GetNumberOfRounds))
        (Variables|Default|SetCurrentRound 1)
        (else
          ;[1 1 1] Check what round it is.
          (if (<= (Variables|Default|GetCurrentRound) (Variables|Default|GetNumberOfRounds))
            (bind _result (Math|Integer|IncrementInt (Variables|Default|GetCurrentRound))
              (:%20%20
                (Variables|Default|SetCurrentRound _result)))))))))

(fn IsEndOfGame
  (if (> (Variables|Default|GetCurrentRound) (Variables|Default|GetNumberOfRounds))
    (return true)
    (else
      (return false))))

(fn ProceedGame
  (bind _bisendofgame (CallFunction|IsEndOfGame))
  (if _bisendofgame
    (Default|CallOnGameEnd)
    (else
      (CallFunction|StartNewRound))))

(fn EndOfRound)

(fn LoadLobby
  (Game|OpenLevel(byName) "Lobby"))

(fn PlayAudio
  (params (VolumeMultiplier :type Float%20%28single-precision%29) (bPersistAcrossLevelTransition :type Boolean))
  ;[1 1 1] Checks if the background music is playing, if not, creates the sound and plays it.
  (Utilities|IsValid (Variables|Default|GetAudio)
    (:Is%20Valid
      (if (not (Audio|Components|Audio|IsPlaying (Variables|Default|GetAudio)))
        (bind _returnvalue (Audio|CreateSound2D "/Game/Audio/Music/BGM_Game.BGM_Game" VolumeMultiplier 1.0 0.0 0 bPersistAcrossLevelTransition :!label _label))
        (bind _output_get (Variables|Default|SetAudio _returnvalue))
        (Audio|Components|Audio|Play _output_get 0.0)))
    (:Is%20Not%20Valid
      (goto _label))))

(fn CreateSaveGameObject
  ;[1 1 1] Sets up the save game file, if the file exists, then the file is loaded. If the file does not exist it is created.
  (bind _returnvalue (SaveGame|DoesSaveGameExist (Variables|Default|GetSaveSlotName)))
  (if _returnvalue
    (bind _returnvalue_2 (SaveGame|LoadGamefromSlot (Variables|Default|GetSaveSlotName)))
    (bind _assave_game_settings (Utilities|Casting|CastToSaveGameSettings _returnvalue_2))
    (Variables|Default|SetSaveGameData _assave_game_settings)
    (else
      (bind _returnvalue_3 (SaveGame|CreateSaveGameObject "/Game/SaveGameSettings/SaveGameSettings.SaveGameSettings_C"))
      (Variables|Default|SetSaveGameData _returnvalue_3))))

(fn SaveOptionsSettings
  (bind _optionswidget (Variables|Default|GetOptionsWidget))
  (bind _savegamedata (Variables|Default|GetSaveGameData))
  ;[1 1 1] This functiion should set the fullscreen mode equal to that of the options setting(which changes with the buttons in the menu).
  ;[1 1 1] Gets the resolution index and the fullscreen mode and (should) save it to the save game object.
  (Variables|/Game/SaveGameSettings/SaveGameSettings.SaveGameSettings_C|SetFullscreenMode_Save _savegamedata (Variables|/Game/Widgets/WBP_Options.WBP_Options_C|GetFullscreen%20Mode _optionswidget))
  (Variables|/Game/Widgets/WBP_Options.WBP_Options_C|SetResolution_index _optionswidget (Variables|/Game/SaveGameSettings/SaveGameSettings.SaveGameSettings_C|GetResolution_index _savegamedata))
  (SaveGame|SaveGametoSlot _savegamedata (Variables|Default|GetSaveSlotName)))

(fn SetSettingsVariables
  (bind _savegamedata (Variables|Default|GetSaveGameData))
  ;[1 1 1] Sets default values for the options menu resolution, fullscreen mode and sound volumes.
  (Variables|/Game/SaveGameSettings/SaveGameSettings.SaveGameSettings_C|SetResolution_index _savegamedata 0)
  (Variables|/Game/SaveGameSettings/SaveGameSettings.SaveGameSettings_C|SetFullscreenMode_Save _savegamedata "Fullscreen")
  (Variables|/Game/SaveGameSettings/SaveGameSettings.SaveGameSettings_C|SetMusicSliderVolume _savegamedata 1.0)
  (Variables|/Game/SaveGameSettings/SaveGameSettings.SaveGameSettings_C|SetSFXSliderVolume _savegamedata 1.0))

(fn LoadSettings
  (bind _returnvalue (SaveGame|DoesSaveGameExist (Variables|Default|GetSaveSlotName)))
  (if _returnvalue
    (SaveGame|LoadGamefromSlot (Variables|Default|GetSaveSlotName))
    (else
      (Development|PrintString "No"))))