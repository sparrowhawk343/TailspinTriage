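; Shared multiplayer camera that follows the active players, starting once GameStarted receives them and appends the BP_LevelMidpoint actor to the list.
; Each tick, it lerps a sphere toward a point halfway between the list's average location and the level midpoint.
; It also loops over each tracked actor, setting spring arm length to the clamped maximum distance to later list entries, so the last iteration overwrites earlier results.
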(event EventTick
  (params (DeltaSeconds :type Float%20%28single-precision%29))
  (if (Variables|Default|GetbGameStarted)
    (CallFunction|CalculateCameraMovement)
    (CallFunction|UpdateSpringArmLength)))

(fn ConstructionScript)

(fn GameStarted
  (params (ActivePlayers :type Array%20of%20BP%20Flying%20Cube%20Object%20References))
  (Variables|Default|SetActivePlayers ActivePlayers)
  (if (not (Utilities|Array|IsEmpty ActivePlayers))
    (bind _returnvalue (Actor|GetActorOfClass "/Game/Blueprints/BP_LevelMidpoint.BP_LevelMidpoint_C"))
    (bind _asactor (Utilities|Casting|CastToActor _returnvalue))
    (Utilities|Array|Add (Variables|Default|GetActivePlayers) _asactor)
    (Variables|Default|SetbGameStarted true)))

(fn CalculateCameraMovement
  (Variables|Default|SetPreviousLocation (Transformation|GetWorldLocation (Variables|Default|GetSphere)))
  (bind _returnvalue (Actor|GetActorOfClass "/Game/Blueprints/BP_LevelMidpoint.BP_LevelMidpoint_C"))
  (bind _returnvalue_2 (Class|GameplayStatics|GetActorArrayAverageLocation (Variables|Default|GetActivePlayers)))
  (Transformation|SetWorldLocation (Variables|Default|GetSphere) (Math|Vector|Lerp(Vector) (Variables|Default|GetPreviousLocation) (/ (+ _returnvalue_2 (Transformation|GetActorLocation _returnvalue)) 2) (Variables|Default|GetFollowSpeed)) false false))

(fn UpdateSpringArmLength
  (bind _activeplayers (Variables|Default|GetActivePlayers))
  (for (_array_element _array_index) _activeplayers
    (Variables|Default|SetCurrentPlayer _array_element)
    (for _index (range (+ _array_index 1) (- (Utilities|Array|Length _activeplayers) 1))
      (Utilities|Array|Add (Variables|Default|GetDistance) (Transformation|GetDistanceTo (Variables|Default|GetCurrentPlayer) (Utilities|Array|Get(acopy) (Variables|Default|GetActivePlayers) _index))))
    (Variables|/Script/Engine.SpringArmComponent|SetTargetArmLength (Variables|Default|GetSpringArm) (Math|Float|Clamp(Float) (.MaxValue (Math|Float|MaxOfFloatArray (Variables|Default|GetDistance))) (Variables|Default|GetMinZoomValue) (Variables|Default|GetMaxZoomValue)))
    (Utilities|Array|Clear (Variables|Default|GetDistance))))